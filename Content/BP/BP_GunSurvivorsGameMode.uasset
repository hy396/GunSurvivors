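; Game mode for GunSurvivors that creates the HUD and drives it from the score.
; On begin play it shows WBP_HUD and binds to a C++-exposed score-changed delegate to refresh the score.
; Whenever the score hits a positive multiple of 1200, it shows the WBP_jiesuan results widget with that score and calls GameStop on the enemy spawner.
; Time-dilation and pause nodes are present but unconnected.
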(event Custom|OnScoreChangedDelegateFired
  (params (NewScore :type Integer))
  ;[1 1 1] 更改得分函数触发委托(UPROPERTY(BlueprintAssignable))委托上加
  (Default|SetScore (Variables|Default|GetHUD) NewScore)
  (if (and (== (Math|Integer|%(Integer) NewScore 1200) 0) (>= (/ NewScore 1200) 1))
    (bind _returnvalue (UserInterface|CreateWidget "/Game/BP/WBP_jiesuan.WBP_jiesuan_C"))
    (UserInterface|Viewport|AddtoViewport _returnvalue 0)
    (Default|SetValue _returnvalue NewScore)
    (bind _returnvalue_2 (Actor|GetActorOfClass "/Game/BP/BP_EnemySpawner.BP_EnemySpawner_C"))
    (Class|EnemySpawner|GameStop _returnvalue_2)))

(event EventBeginPlay
  (bind _returnvalue (UserInterface|CreateWidget "/Game/BP/WBP_HUD.WBP_HUD_C"))
  (bind _output_get (Variables|Default|SetHUD _returnvalue))
  (UserInterface|Viewport|AddtoViewport _output_get 0)
  (Default|SetScore (Variables|Default|GetHUD))
  (EventDispatchers|BindEventtoScoreChangedDelegate (delegate Custom|OnScoreChangedDelegateFired)))

(event EventTick
  (params (DeltaSeconds :type Float%20%28single-precision%29)))

(fn ConstructionScript)