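; BP_Enemy1 is an enemy that ends play on contact, apparently for the beginner (Xinshou) tutorial.
; Its capsule overlap shows the WBP_Xinshou_end widget when hit by a BP_Bullet, or WBP_Over2 when touching BP_Player.
; Both branches then set the HUD's Op flag to false through BP_GunSurvivorsGameMode.
; The Blueprint itself contains no movement, damage or destroy logic.
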(event OnComponentBeginOverlap(CapsuleComp)
  (params (OverlappedComponent :type Primitive%20Component%20Object%20Reference) (OtherActor :type Actor%20Object%20Reference) (OtherComp :type Primitive%20Component%20Object%20Reference) (OtherBodyIndex :type Integer) (bFromSweep :type Boolean) (SweepResult :type Hit%20Result%20Structure%20%28by%20ref%29))
  (Utilities|FlowControl|Sequence
    (:then_0
      (bind _asbp_bullet (Utilities|Casting|CastToBP_Bullet OtherActor))
      (Utilities|IsValid _asbp_bullet
        (:Is%20Valid
          (bind _returnvalue (UserInterface|CreateWidget "/Game/BP/WBP_Xinshou_end.WBP_Xinshou_end_C"))
          (UserInterface|Viewport|AddtoViewport _returnvalue 0))))
    (:then_1
      (bind _asbp_player (Utilities|Casting|CastToBP_Player OtherActor))
      (Utilities|IsValid _asbp_player
        (:Is%20Valid
          (bind _returnvalue_2 (UserInterface|CreateWidget "/Game/BP/WBP_Over2.WBP_Over2_C"))
          (UserInterface|Viewport|AddtoViewport _returnvalue_2 0)))))
  (bind _asbp_gun_survivors_game_mode (Utilities|Casting|CastToBP_GunSurvivorsGameMode (Game|GetGameMode)))
  (Variables|/Game/BP/WBP_HUD.WBP_HUD_C|Setop (Variables|/Game/BP/BP_GunSurvivorsGameMode.BP_GunSurvivorsGameMode_C|GetHUD _asbp_gun_survivors_game_mode) false))

(event EventBeginPlay)

(event Collision|EventActorBeginOverlap
  (params (OtherActor :type Actor%20Object%20Reference)))

(event EventTick
  (params (DeltaSeconds :type Float%20%28single-precision%29)))

(fn ConstructionScript)